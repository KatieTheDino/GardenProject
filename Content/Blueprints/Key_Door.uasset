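; Key_Door is a door Blueprint that slides open once the player's FirstPersonCharacter has exactly two Points.
; BeginPlay caches the player character, and Tick polls its Points every frame to play a timeline.
; The timeline lerps the relative location of both the scene root and the Cube between start and end position variables.
; Overlap plays no part, as that event is an empty, disabled stub.
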(event EventBeginPlay
  (bind _asfirst_person_character (Utilities|Casting|CastToFirstPersonCharacter (Game|Player|GetPlayerPawn 0)))
  (Variables|Default|SetMyCharacter _asfirst_person_character))

(event Collision|EventActorBeginOverlap
  (params (OtherActor :type Actor%20Object%20Reference))
  ;[1 1 1] Makes door open
)

(event EventTick
  (params (DeltaSeconds :type Float%20%28single-precision%29))
  ;[1 1 1] Makes door open
  (if (== (Variables|/Game/FirstPersonBP/Blueprints/FirstPersonCharacter.FirstPersonCharacter_C|GetPoints (Variables|Default|GetMyCharacter)) 2)
    (bind _opensesame (Timeline|Timeline_0 Play)
      (:Update
        (Transformation|SetRelativeLocation (Variables|Default|GetDefaultSceneRoot) (Math|Vector|Lerp(Vector) (Variables|Default|GetPositioNStart) (Variables|Default|GetPosiotnEnd) _opensesame) false false)))))

(fn ConstructionScript)